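; BP_GridPath builds a tile grid with an instanced mesh floor in its construction script.
; TileType maps each tile index, packed as X * 1000 + Y, to a location offset spaced by TileSize.
; Existing NextAearTile direction keys get the middle tile of their matching edge, apparently as links to neighboring areas.
; Tile Vaild checks whether an index exists in the grid; no pathfinding logic is present.
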(event `self.ReceiveBeginPlay`)

(event `self.ReceiveTick`
  (params (DeltaSeconds :type "Float (single-precision)")))

(fn `UserConstructionScript`
  (locals (`Line Material` :type "MaterialInstanceDynamic Object Reference") (`Selection Material` :type "MaterialInstanceDynamic Object Reference") (`Line Start` :type "Float (double-precision)") (`Line End` :type "Float (double-precision)") (`Line Vectices` :type "Array of Vector Structure") (`Line Triangles` :type "Array of Integer") (`Selection Vectices` :type "Array of Vector Structure") (`Selection Triangles` :type "Array of Integer"))
  (bind _next_aear_tile (`self.Next Aear Tile`))
  (bind _grid_row (`self.Grid Row`))
  (bind _returnvalue (- (`self.Grid Row`) 1))
  (bind _returnvalue_2 (- (`self.Grid Column`) 1))
  (bind _returnvalue_3 (/ (`self.TileSize`) 400.0))
  (bind _returnvalue_4 (`KismetMathLibrary.FFloor` (`self.TileSize`)))
  (bind _returnvalue_5 (/ _returnvalue_2 2))
  (bind _returnvalue_6 (* (/ _returnvalue 2) 1000))
  (`|ExecutionSequence`
    (:`then_0`
      ;[1 1 1] Set Up Grid Data
      (`|ExecutionSequence`
        (:`then_0`
          (for _index (range (* (`self.Grid Row`) (`self.Grid Column`)))
            (`BlueprintMapLibrary.Map_Add` (`self.Tile_Type`) (+ (/ _index _grid_row) (* (mod _index _grid_row) 1000)) (`KismetMathLibrary.MakeVector` (`KismetMathLibrary.Conv_IntToDouble` (* (mod _index _grid_row) _returnvalue_4)) (`KismetMathLibrary.Conv_IntToDouble` (* (/ _index _grid_row) _returnvalue_4))))))
        (:`then_1`
          (if (> (`BlueprintMapLibrary.Map_Length` _next_aear_tile) 0)
            (bind _keys (`BlueprintMapLibrary.Map_Keys` _next_aear_tile))
            (for _array_element _keys
              (switch `/Game/Blueprints/Direction` _array_element
                (:`NewEnumerator0`
                  (`BlueprintMapLibrary.Map_Add` (`self.Next Aear Tile`) _array_element _returnvalue_6))
                (:`NewEnumerator2`
                  (`BlueprintMapLibrary.Map_Add` (`self.Next Aear Tile`) _array_element (+ (* _returnvalue 1000) _returnvalue_5)))
                (:`NewEnumerator4`
                  (`BlueprintMapLibrary.Map_Add` (`self.Next Aear Tile`) _array_element (+ _returnvalue_6 _returnvalue_2)))
                (:`NewEnumerator6`
                  (`BlueprintMapLibrary.Map_Add` (`self.Next Aear Tile`) _array_element _returnvalue_5))))))))
    (:`then_1`
      ;[1 1 1] Creat Grid Floor
      (bind _values (`BlueprintMapLibrary.Map_Values` (`self.Tile_Type`)))
      (for _array_element_2 _values
        (`InstancedStaticMeshComponent.AddInstance` (`self.Grid_Floor`) (`KismetMathLibrary.MakeTransform` _array_element_2 (struct) (`KismetMathLibrary.MakeVector` _returnvalue_3 _returnvalue_3 0.5)))))))